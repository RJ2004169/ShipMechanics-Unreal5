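; BP_Ship is a sailing ship that drives itself along its mesh's forward vector every tick while the sail is down.
; The R key flip-flops the sail state and updates the player character's sail prompt text.
; Ladder and wheel colliders cast overlapping actors to BP_ThirdPersonCharacter to toggle climbing, restore walking on ladder exit, and show or clear the take-control prompt.
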(event `self.ReceiveTick`
  (params (DeltaSeconds :type "Float (single-precision)"))
  (if (not (`self.sailUp`))
    (`self.AddMovementInput` (`SceneComponent.GetForwardVector` (`self.StaticMesh`)) 10.0)))

(event `Key|R`
  (params (Key :type "Key Structure"))
  (bind _returnvalue (`GameplayStatics.GetPlayerCharacter` 0))
  (:`Pressed`
    (`/Engine/EditorBlueprintResources/StandardMacros.FlipFlop`
      (:`A`
        (set `self.sailUp` false)
        (bind _asbp_third_person_character (cast `/Game/ThirdPerson/Blueprints/BP_ThirdPersonCharacter` _returnvalue))
        (set `/Game/ThirdPerson/Blueprints/BP_ThirdPersonCharacter.SailUpDownText` "Press R to Tie Up Sail" _asbp_third_person_character))
      (:`B`
        (set `self.sailUp` true)
        (bind _asbp_third_person_character_2 (cast `/Game/ThirdPerson/Blueprints/BP_ThirdPersonCharacter` _returnvalue))
        (set `/Game/ThirdPerson/Blueprints/BP_ThirdPersonCharacter.SailUpDownText` "Press R to Let Down Sail" _asbp_third_person_character_2)))))

(event `self.ladderCollider.OnComponentBeginOverlap`
  (params (OverlappedComponent :type "PrimitiveComponent Object Reference") (OtherActor :type "Actor Object Reference") (OtherComp :type "PrimitiveComponent Object Reference") (OtherBodyIndex :type Integer) (bFromSweep :type Boolean) (SweepResult :type "HitResult Structure (by ref)"))
  (bind _asbp_third_person_character (cast `/Game/ThirdPerson/Blueprints/BP_ThirdPersonCharacter` OtherActor))
  (set `/Game/ThirdPerson/Blueprints/BP_ThirdPersonCharacter.climbLadder` true _asbp_third_person_character))

(event `self.ladderCollider.OnComponentEndOverlap`
  (params (OverlappedComponent :type "PrimitiveComponent Object Reference") (OtherActor :type "Actor Object Reference") (OtherComp :type "PrimitiveComponent Object Reference") (OtherBodyIndex :type Integer))
  (bind _asbp_third_person_character (cast `/Game/ThirdPerson/Blueprints/BP_ThirdPersonCharacter` OtherActor))
  (set `/Game/ThirdPerson/Blueprints/BP_ThirdPersonCharacter.climbLadder` false _asbp_third_person_character)
  (`CharacterMovementComponent.SetMovementMode` (`Character.CharacterMovement` _asbp_third_person_character) "MOVE_Walking" 0))

(event `self.wheelCollider.OnComponentBeginOverlap`
  (params (OverlappedComponent :type "PrimitiveComponent Object Reference") (OtherActor :type "Actor Object Reference") (OtherComp :type "PrimitiveComponent Object Reference") (OtherBodyIndex :type Integer) (bFromSweep :type Boolean) (SweepResult :type "HitResult Structure (by ref)"))
  (bind _asbp_third_person_character (cast `/Game/ThirdPerson/Blueprints/BP_ThirdPersonCharacter` OtherActor))
  (set `/Game/ThirdPerson/Blueprints/BP_ThirdPersonCharacter.UIInteractText` "Press E to Take Control" _asbp_third_person_character))

(event `self.wheelCollider.OnComponentEndOverlap`
  (params (OverlappedComponent :type "PrimitiveComponent Object Reference") (OtherActor :type "Actor Object Reference") (OtherComp :type "PrimitiveComponent Object Reference") (OtherBodyIndex :type Integer))
  (bind _asbp_third_person_character (cast `/Game/ThirdPerson/Blueprints/BP_ThirdPersonCharacter` OtherActor))
  (set `/Game/ThirdPerson/Blueprints/BP_ThirdPersonCharacter.UIInteractText` "" _asbp_third_person_character))

(fn `UserConstructionScript`)